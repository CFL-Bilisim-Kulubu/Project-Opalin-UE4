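; Scene capture actor that follows the player to record tagged grass affectors, apparently for particle-based foliage interaction.
; Each tick it snaps its XY to the capture's pixel world size, stays above the player and writes its location to MPC_Capture.
; BeginPlay and UpdateShowOnly add GrassAffector-tagged components to the show-only list and flag overlapping characters' trail sources in range.
; Box overlaps toggle InRange on TrailSource-tagged actors.
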(event `self.Box.OnComponentEndOverlap`
  (params (OverlappedComponent :type "PrimitiveComponent Object Reference") (OtherActor :type "Actor Object Reference") (OtherComp :type "PrimitiveComponent Object Reference") (OtherBodyIndex :type Integer))
  ;[1 1 1] End Overlap
  (if (`self.ActorHasTag` OtherActor "TrailSource")
    (set `/Game/ParticleBasedFoliageInteraction/Blueprints/TrailSourceComponent.InRange` false (`self.GetComponentByClass` OtherActor "/Game/ParticleBasedFoliageInteraction/Blueprints/TrailSourceComponent.TrailSourceComponent_C"))))

(event `self.Box.OnComponentBeginOverlap`
  (params (OverlappedComponent :type "PrimitiveComponent Object Reference") (OtherActor :type "Actor Object Reference") (OtherComp :type "PrimitiveComponent Object Reference") (OtherBodyIndex :type Integer) (bFromSweep :type Boolean) (SweepResult :type "HitResult Structure (by ref)"))
  ;[1 1 1] Begin Overlap
  (if (`self.ActorHasTag` OtherActor "TrailSource")
    (set `/Game/ParticleBasedFoliageInteraction/Blueprints/TrailSourceComponent.InRange` true (`self.GetComponentByClass` OtherActor "/Game/ParticleBasedFoliageInteraction/Blueprints/TrailSourceComponent.TrailSourceComponent_C"))))

(event `self.ReceiveTick`
  (params (DeltaSeconds :type "Float (single-precision)"))
  ;[1 1 1] Event Tick
  (`self.Move Capture`))

(event `self.ReceiveBeginPlay`
  ;[1 1 1] Update List
  (bind _outactors (`GameplayStatics.GetAllActorsWithTag` "GrassAffector" :!label _label))
  (for _array_element _outactors
    (for _array_element_2 (`self.GetComponentsByTag` _array_element "/Script/Engine.PrimitiveComponent" "GrassAffector")
      (`SceneCaptureComponent.ShowOnlyComponent` (`self.SceneCapture`) _array_element_2)
      (for _array_element_3 (`PrimitiveComponent.GetOverlappingActors` (`self.Box`) "/Script/Engine.Character")
        (set `/Game/ParticleBasedFoliageInteraction/Blueprints/TrailSourceComponent.InRange` true (`self.GetComponentByClass` _array_element_3 "/Game/ParticleBasedFoliageInteraction/Blueprints/TrailSourceComponent.TrailSourceComponent_C"))))))

(event `/Game/AdvancedLocomotionV3/Blueprints/ALS_Interface.UpdateShowOnly`
  ;[1 1 1] Update List
  (goto _label))

(fn `Move Capture`
  (locals (`Move Offset X` :type "Float (double-precision)") (`Move Offset Y` :type "Float (double-precision)"))
  (bind (_returnvalue_x _returnvalue_y) (`KismetMathLibrary.BreakVector` (`self.K2_GetActorLocation`)))
  (bind (_returnvalue_x_2 _returnvalue_y_2) (`KismetMathLibrary.BreakVector` (`self.K2_GetActorLocation` (`GameplayStatics.GetPlayerCharacter` 0))))
  (bind (_returnvalue_x_3 _returnvalue_y_3 _returnvalue_z) (`KismetMathLibrary.BreakVector` (`self.K2_GetActorLocation` (`GameplayStatics.GetPlayerCharacter` 0))))
  (bind _returnvalue (`KismetMaterialLibrary.GetScalarParameterValue` "/Game/ParticleBasedFoliageInteraction/MPC_Capture.MPC_Capture" "CaptureSize"))
  (bind (_returnvalue_x_4 _returnvalue_y_4) (`KismetMathLibrary.BreakVector` (- (`self.SnapToPixelWorldSize` _returnvalue_x_2 _returnvalue_y_2 (* (/ 1.0 _returnvalue) (`SceneCaptureComponent2D.OrthoWidth` (`self.SceneCapture`)))) (`self.K2_GetActorLocation`))))
  (bind _output_get (set `local.Move Offset X` _returnvalue_x_4))
  (bind _output_get_2 (set `local.Move Offset Y` _returnvalue_y_4))
  (`self.K2_AddActorWorldOffset` (`KismetMathLibrary.MakeVector` _output_get _output_get_2))
  (`self.K2_SetActorLocation` (`KismetMathLibrary.MakeVector` _returnvalue_x _returnvalue_y (+ _returnvalue_z 512.0)))
  (`KismetMaterialLibrary.SetVectorParameterValue` "/Game/ParticleBasedFoliageInteraction/MPC_Capture.MPC_Capture" "CaptureLocation" (`KismetMathLibrary.Conv_VectorToLinearColor` (`self.K2_GetActorLocation`)))
  (return))

(fn `UserConstructionScript`)