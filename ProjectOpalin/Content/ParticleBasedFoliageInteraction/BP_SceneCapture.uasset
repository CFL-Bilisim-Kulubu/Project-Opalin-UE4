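; Scene capture actor for particle-based foliage interaction that follows the player and captures only components tagged GrassAffector.
; BeginPlay and UpdateShowOnly add tagged primitives from tagged actors to the show-only list.
; Each tick, MoveCapture snaps XY to the capture's texel grid, derived from ortho width and CaptureSize, and holds a fixed height above the player.
; It publishes CaptureLocation to MPC_Capture for materials.
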(event `self.ReceiveTick`
  (params (DeltaSeconds :type "Float (single-precision)"))
  (`self.Move Capture`))

(event `self.ReceiveBeginPlay`
  (bind _outactors (`GameplayStatics.GetAllActorsWithTag` "GrassAffector" :!label _label))
  (for _array_element _outactors
    (for _array_element_2 (`self.GetComponentsByTag` _array_element "/Script/Engine.PrimitiveComponent" "GrassAffector")
      (`SceneCaptureComponent.ShowOnlyComponent` (`self.SceneCapture`) _array_element_2))))

(event `/Game/AdvancedLocomotionV3/Blueprints/ALS_Interface.UpdateShowOnly`
  (goto _label))

(fn `Move Capture`
  (locals (`Move Offset X` :type "Float (double-precision)") (`Move Offset Y` :type "Float (double-precision)"))
  (bind (_returnvalue_x _returnvalue_y) (`KismetMathLibrary.BreakVector` (`self.K2_GetActorLocation`)))
  (bind (_returnvalue_x_2 _returnvalue_y_2) (`KismetMathLibrary.BreakVector` (`self.K2_GetActorLocation` (`GameplayStatics.GetPlayerCharacter` 0))))
  (bind (_returnvalue_x_3 _returnvalue_y_3 _returnvalue_z) (`KismetMathLibrary.BreakVector` (`self.K2_GetActorLocation` (`GameplayStatics.GetPlayerCharacter` 0))))
  (bind _returnvalue (`KismetMaterialLibrary.GetScalarParameterValue` "/Game/ParticleBasedFoliageInteraction/MPC_Capture.MPC_Capture" "CaptureSize"))
  (bind (_returnvalue_x_4 _returnvalue_y_4) (`KismetMathLibrary.BreakVector` (- (`self.SnapToPixelWorldSize` _returnvalue_x_2 _returnvalue_y_2 (* (/ 1.0 _returnvalue) (`SceneCaptureComponent2D.OrthoWidth` (`self.SceneCapture`)))) (`self.K2_GetActorLocation`))))
  (bind _output_get (set `local.Move Offset X` _returnvalue_x_4))
  (bind _output_get_2 (set `local.Move Offset Y` _returnvalue_y_4))
  (`self.K2_AddActorWorldOffset` (`KismetMathLibrary.MakeVector` _output_get _output_get_2))
  (`self.K2_SetActorLocation` (`KismetMathLibrary.MakeVector` _returnvalue_x _returnvalue_y (+ _returnvalue_z 512.0)))
  (`KismetMaterialLibrary.SetVectorParameterValue` "/Game/ParticleBasedFoliageInteraction/MPC_Capture.MPC_Capture" "CaptureLocation" (`KismetMathLibrary.Conv_VectorToLinearColor` (`self.K2_GetActorLocation`)))
  (return))

(fn `UserConstructionScript`)