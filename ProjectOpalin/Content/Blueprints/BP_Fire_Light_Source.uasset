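; Fire light source Blueprint that makes a point light flicker and wander like firelight.
; A looping timer frequently picks a random offset within an upward cone, scaled by a max range, and a random intensity around the base value.
; Tick smoothly interpolates the light's relative location and intensity toward those targets at a shared speed.
; The construction script applies the base intensity to the light.
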(event `self.ReceiveBeginPlay`
  (`KismetSystemLibrary.K2_SetTimer` null "Randomize" 0.07 true))

(event `self.ReceiveTick`
  (params (DeltaSeconds :type "Float (single-precision)"))
  (bind _pointlight (`self.PointLight`))
  (`SceneComponent.K2_SetRelativeLocation` (`self.PointLight`) (`KismetMathLibrary.VInterpTo` (`SceneComponent.RelativeLocation` (`self.PointLight`)) (`self.DesiredLocation`) DeltaSeconds (`self.Speed`)) false false)
  (`LightComponent.SetIntensity` _pointlight (`KismetMathLibrary.FInterpTo` (`LightComponentBase.Intensity` _pointlight) (`self.DesiredIntensity`) DeltaSeconds (`self.Speed`))))

(fn `Randomize`
  (bind _intensityrange (`self.IntensityRange`))
  (set `self.DesiredLocation` (* (`KismetMathLibrary.RandomUnitVectorInConeInRadians` (0.0 0.0 1.0) 50.0) (`self.MaxRange`)))
  (set `self.DesiredIntensity` (+ (`self.LightIntensity`) (`KismetMathLibrary.RandomFloatInRange` (* _intensityrange -1.0) _intensityrange))))

(fn `UserConstructionScript`
  (`LightComponent.SetIntensity` (`self.PointLight`) (`self.LightIntensity`)))