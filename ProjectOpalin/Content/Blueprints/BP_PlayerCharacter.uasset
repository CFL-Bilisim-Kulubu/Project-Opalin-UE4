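; Player character Blueprint that manages trail particle emitters tagged as GrassAffector for every actor tagged TrailSource.
; On BeginPlay it adds an emitter per source from its TrailSourceComponent settings and attaches it to that actor's capsule.
; Emitters start inactive and owner-no-see, then the first BP_SceneCapture is told to update its show-only list.
; Each tick syncs every emitter's active state to its source's TrailEnebled flag.
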(event `/Game/AdvancedLocomotionV3/Blueprints/ALS_Interface.BeginPlay`
  ;[1 0.07016 0.03035] Interface Begin Play
  (`self.Update Trail Sources`))

(event `/Game/AdvancedLocomotionV3/Blueprints/ALS_Interface.Tick`
  ;[1 0.07016 0.03035] Interface Tick
  (`self.Update Trail States`))

(event `/Game/AdvancedLocomotionV3/Blueprints/ALS_Interface.DropOnGround`
  ;[1 0.07016 0.03035] Interface On Landed
)

(fn `Update Trail Sources`
  ;[1 1 1] Update Trail Sources
  (bind _outactors (`GameplayStatics.GetAllActorsWithTag` "TrailSource"))
  (for _array_element _outactors
    (bind _returnvalue (`self.GetComponentByClass` _array_element "/Game/Blueprints/FoliageInteraction/TrailSourceComponent.TrailSourceComponent_C"))
    (`KismetArrayLibrary.Array_Add` (`self.TrailSources`) _returnvalue)
    (bind _returnvalue_2 (`AddComponent|NODE_AddParticleSystemComponent-0` :`self` self :`RelativeTransform` (`KismetMathLibrary.MakeTransform` (`/Game/Blueprints/FoliageInteraction/TrailSourceComponent.SourceOffset` _returnvalue))))
    (bind _returnvalue_3 (`SceneComponent.K2_AttachToComponent` _returnvalue_2 (`self.GetComponentByClass` _array_element "/Script/Engine.CapsuleComponent") "None" "KeepRelative" "KeepWorld" "KeepWorld" true))
    (`ParticleSystemComponent.SetTemplate` _returnvalue_2 (`/Game/Blueprints/FoliageInteraction/TrailSourceComponent.Emitter Template` _returnvalue))
    (`KismetArrayLibrary.Array_Add` (`self.TrailEmitters`) _returnvalue_2)
    (`ActorComponent.Deactivate` _returnvalue_2)
    (set `ActorComponent.ComponentTags` (`|MakeArray` "GrassAffector" :!type "Name") _returnvalue_2)
    (`PrimitiveComponent.SetOwnerNoSee` _returnvalue_2 true)
    (`KismetSystemLibrary.PrintString` (`KismetStringLibrary.Concat_StrStr` (`KismetStringLibrary.Concat_StrStr` "Trail Spawned / Owner: " (`KismetSystemLibrary.GetDisplayName` (`ActorComponent.GetOwner` _returnvalue_2))) (`KismetStringLibrary.Concat_StrStr` " / Attach: " (select `bool` _returnvalue_3 :`false` "Fail" :`true` "Succses"))) true true (struct :`R` 0.036079 :`G` 0.630208 :`A` 1.0) 10.0))
  (bind _outactors_2 (`GameplayStatics.GetAllActorsOfClass` "/Game/Blueprints/FoliageInteraction/BP_SceneCapture.BP_SceneCapture_C"))
  (message `/Game/AdvancedLocomotionV3/Blueprints/ALS_Interface.UpdateShowOnly` (`|GetArrayItem` _outactors_2)))

(fn `Update Trail States`
  ;[1 1 1] Update Trail States
  (for (_array_element _array_index) (`self.TrailSources`)
    (bind _astrail_source_component (cast `/Game/Blueprints/FoliageInteraction/TrailSourceComponent` _array_element))
    (`ActorComponent.SetActive` (`|GetArrayItem` (`self.TrailEmitters`) _array_index) (`/Game/Blueprints/FoliageInteraction/TrailSourceComponent.TrailEnebled` _astrail_source_component) false)))

(fn `UserConstructionScript`
  (`parent.UserConstructionScript`))