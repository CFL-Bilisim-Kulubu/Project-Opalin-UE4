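; Foliage capture actor that follows player 0 with an orthographic scene capture of grass affectors, likely for foliage interaction.
; On BeginPlay it adds primitive components tagged GrassAffector, on actors with that tag, to the capture's show-only list.
; Each Tick it moves in XY, snapped to texel-sized world steps derived from OrthoWidth and MPC_Capture's CaptureSize.
; It then writes its position to CaptureLocation in MPC_Capture for materials.
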(event `self.ReceiveTick`
  (params (DeltaSeconds :type "Float (single-precision)"))
  (`self.Move Capture`))

(event `self.ReceiveBeginPlay`
  (bind _outactors (`GameplayStatics.GetAllActorsWithTag` "GrassAffector"))
  (for _array_element _outactors
    (for _array_element_2 (`self.GetComponentsByTag` _array_element "/Script/Engine.PrimitiveComponent" "GrassAffector")
      (`SceneCaptureComponent.ShowOnlyComponent` (`self.SceneCapture`) _array_element_2)))
  (`KismetSystemLibrary.PrintString` "Done"))

(fn `Move Capture`
  (locals (`Move Offset X` :type "Float (double-precision)") (`Move Offset Y` :type "Float (double-precision)"))
  (bind (_returnvalue_x _returnvalue_y) (`KismetMathLibrary.BreakVector` (`self.K2_GetActorLocation` (`GameplayStatics.GetPlayerCharacter` 0))))
  (bind _returnvalue (`KismetMaterialLibrary.GetScalarParameterValue` "/Game/RenderTarget/MPC_Capture.MPC_Capture" "CaptureSize"))
  (bind (_returnvalue_x_2 _returnvalue_y_2) (`KismetMathLibrary.BreakVector` (- (`self.SnapToPixelWorldSize` _returnvalue_x _returnvalue_y (* (/ 1.0 _returnvalue) (`SceneCaptureComponent2D.OrthoWidth` (`self.SceneCapture`)))) (`self.K2_GetActorLocation`))))
  (bind _output_get (set `local.Move Offset X` _returnvalue_x_2))
  (bind _output_get_2 (set `local.Move Offset Y` _returnvalue_y_2))
  (`self.K2_AddActorWorldOffset` (`KismetMathLibrary.MakeVector` _output_get _output_get_2))
  (`KismetMaterialLibrary.SetVectorParameterValue` "/Game/RenderTarget/MPC_Capture.MPC_Capture" "CaptureLocation" (`KismetMathLibrary.Conv_VectorToLinearColor` (`self.K2_GetActorLocation`)))
  (return))

(fn `UserConstructionScript`)